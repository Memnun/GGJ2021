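; McGuffing is the objective pickup that switches the top-down game into its escape phase.
; On BeginPlay it registers itself as the player character's CurrentGoal.
; InitializePowerup starts the game mode's Go Mode, retargets the collecting player's goal to the level's ExfilPoint and shows a progress message sending them to the Segway.
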(event `self.ReceiveBeginPlay`
  (`parent.ReceiveBeginPlay`)
  (bind _astop_down_character (cast `/Game/TopDownBP/Blueprints/TopDownCharacter` (`GameplayStatics.GetPlayerPawn` 0)))
  (set `/Game/TopDownBP/Blueprints/TopDownCharacter.CurrentGoal` self _astop_down_character))

(event `self.InitializePowerup`
  (params (Player :type "/Game/TopDownBP/Blueprints/TopDownCharacter Object Reference"))
  (bind _astop_down_game_mode (cast `/Game/TopDownBP/Blueprints/TopDownGameMode` (`GameplayStatics.GetGameMode`)))
  (`/Game/TopDownBP/Blueprints/TopDownGameMode.StartGoMode` _astop_down_game_mode)
  (bind _returnvalue (`GameplayStatics.GetActorOfClass` "/Game/Blueprints/Pickups/ExfilPoint.ExfilPoint_C"))
  (set `/Game/TopDownBP/Blueprints/TopDownCharacter.CurrentGoal` _returnvalue Player)
  (bind _returnvalue_2 (`|CreateWidget` "/Game/UI/MidGame/ProgressMessage.ProgressMessage_C" null "GET TO THE SEGWAY"))
  (`UserWidget.AddToViewport` _returnvalue_2 0))

(fn `UserConstructionScript`
  (`parent.UserConstructionScript`))