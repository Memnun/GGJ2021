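; Guard AI controller that starts the guard behavior tree and feeds its blackboard.
; On BeginPlay it runs BT_Guard_Master and stores the first player character under the Player key.
; A SoundHeard event, given a location, flags HeardSound and writes that location to LastKnownPosition when the blackboard is valid.
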(event `self.ReceiveBeginPlay`
  (`self.RunBehaviorTree` self "/Game/Blueprints/AI/BT_Guard_Master.BT_Guard_Master")
  (`BlackboardComponent.SetValueAsObject` (`AIBlueprintHelperLibrary.GetBlackboard` self) "Player" (`GameplayStatics.GetPlayerCharacter` 0)))

(event `SoundHeard`
  (params (SoundLocation :type "Vector Structure"))
  (bind _returnvalue (`AIBlueprintHelperLibrary.GetBlackboard` self))
  (`/Engine/EditorBlueprintResources/StandardMacros.IsValid` _returnvalue
    (:`Is Valid`
      (`BlackboardComponent.SetValueAsBool` _returnvalue "HeardSound" true)
      (`BlackboardComponent.SetValueAsVector` _returnvalue "LastKnownPosition" SoundLocation))))

(fn `UserConstructionScript`)