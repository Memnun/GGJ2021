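; Patrol guard NPC that switches bark audio between wandering, seeking and player-spotted states, and plays footstep sounds.
; A single attached bark sound is driven by a parameter from state events.
; Heard noises go to GuardAIController unless the player is already seen.
; Tick draws debug sight text and last-known-position sphere, scales an optional sound-radius display with speed, and aligns a cone to eye yaw at fixed height.
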(event `self.ReceiveBeginPlay`
  (add `self.PlayerSpotted` (delegate `PlayerSpotted_Event`))
  (bind _returnvalue (`FMODBlueprintStatics.PlayEventAttached` "/Game/FMOD/Events/NPC/GuardBark.GuardBark" (`self.Mesh`) "None" (0.0 0.0 0.0) "KeepRelativeOffset" false true false))
  (bind _output_get (set `self.GuardBarkSound` _returnvalue))
  (`FMODAudioComponent.SetParameter` _output_get (`self.GuardBarkParam`) 0.0))

(event `PlayerSpotted_Event`
  (bind _guardbarksound (`self.GuardBarkSound`)
    (:`then`
      (`FMODAudioComponent.SetParameter` _guardbarksound (`self.GuardBarkParam`) 2.0))
    (:`else`)))

(event `ResumeWander`
  (bind _guardbarksound (`self.GuardBarkSound`)
    (:`then`
      (`FMODAudioComponent.SetParameter` _guardbarksound (`self.GuardBarkParam`) 0.0)
      (`FMODAudioComponent.Play` _guardbarksound))
    (:`else`)))

(event `BeginSeeking`
  (bind _guardbarksound (`self.GuardBarkSound`)
    (:`then`
      (`FMODAudioComponent.SetParameter` _guardbarksound (`self.GuardBarkParam`) 1.0)
      (`FMODAudioComponent.Play` _guardbarksound))
    (:`else`)))

(event `SetSoundDisplayEnabled`
  (params (Enabled :type Boolean))
  (bind _output_get (set `self.SoundDisplayEnabled` Enabled))
  (`SceneComponent.SetVisibility` (`self.SoundRadius`) _output_get false))

(event `self.ReceiveTick`
  (params (DeltaSeconds :type "Float (single-precision)"))
  (bind (_eyetransform_location _eyetransform_rotation) (`KismetMathLibrary.BreakTransform` (`self.GetEyeTransform`)))
  (bind _returnvalue (`AIBlueprintHelperLibrary.GetBlackboard` (`AIBlueprintHelperLibrary.GetAIController` self)))
  (`parent.ReceiveTick` DeltaSeconds)
  (`KismetSystemLibrary.DrawDebugString` (`SceneComponent.GetSocketLocation` (`self.Mesh`) "head") (`KismetMathLibrary.SelectString` "Doo doo doo I See You" "WHERE ARE THEY" (`self.HasSeenPlayer`)) null)
  (`/Engine/EditorBlueprintResources/StandardMacros.IsValid` _returnvalue
    (:`Is Valid`
      (`KismetSystemLibrary.DrawDebugSphere` (`BlackboardComponent.GetValueAsVector` _returnvalue "LastKnownPosition") 20.0 12 (struct :`R` 1.0 :`G` 1.0 :`B` 1.0 :`A` 1.0) 0.0 5.0)
      (`self.UpdateSoundRadius`)
      (`SceneComponent.K2_SetWorldTransform` (`self.ConeRoot`) (`KismetMathLibrary.MakeTransform` (`KismetMathLibrary.MakeVector` (.x _eyetransform_location) (.y _eyetransform_location) 1310.0) (`KismetMathLibrary.MakeRotator` 0.0 0.0 (.yaw _eyetransform_rotation))) false false))))

(event `SoundHeard`
  (params (Location :type "Vector Structure"))
  (if (not (`self.HasSeenPlayer`))
    (bind _asguard_aicontroller (cast `/Game/Blueprints/AI/GuardAIController` (`AIBlueprintHelperLibrary.GetAIController` self)))
    (`/Game/Blueprints/AI/GuardAIController.SoundHeard` _asguard_aicontroller Location)))

(event `/Game/Blueprints/AnimNotifyInterface.Step`
  (bind _returnvalue (`FMODBlueprintStatics.PlayEventAttached` "/Game/FMOD/Events/NPC/FootstepGuard.FootstepGuard" (`self.Mesh`) "None" (0.0 0.0 0.0) "KeepRelativeOffset"))
  (`FMODAudioComponent.Release` _returnvalue))

(fn `GetEyeTransform`
  (returns (EyeTransform :type "Transform Structure"))
  (return (`SceneComponent.GetSocketTransform` (`self.Mesh`) "eyes" "RTS_World")))

(fn `UpdateSoundRadius`
  (bind _currentsoundradius (`self.CurrentSoundRadius`))
  (if (`self.SoundDisplayEnabled`)
    (set `self.CurrentSoundRadius` (* (`KismetMathLibrary.NormalizeToRange` (`KismetMathLibrary.VSize` (`self.GetVelocity`)) 0.0 (`MovementComponent.GetMaxSpeed` (`self.CharacterMovement`))) (`self.MaxSoundRadius`)))
    (`SceneComponent.SetWorldScale3D` (`self.SoundRadius`) (`KismetMathLibrary.MakeVector` 1.0 _currentsoundradius _currentsoundradius))))

(fn `UserConstructionScript`)