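; Security camera that sweeps its head back and forth and relays player sightings to nearby patrol guards.
; A ping-pong timeline drives the yaw, with speed set through the actor's custom time dilation.
; A communication sphere tracks guards in range, adding or removing the camera as their sight source as the player is spotted or lost.
; Detection uses inherited events and the lens socket as eye; Tick prints the guard count for debugging.
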(event `self.ReceiveTick`
  (params (DeltaSeconds :type "Float (single-precision)"))
  (`parent.ReceiveTick` DeltaSeconds)
  (`KismetSystemLibrary.DrawDebugString` (`self.K2_GetActorLocation`) (`KismetStringLibrary.Conv_IntToString` (`KismetArrayLibrary.Array_Length` (`self.PatrolGuardsInRange`))) null (struct :`G` 0.087367 :`B` 1.0 :`A` 1.0) 0.034))

(event `self.ReceiveBeginPlay`
  (add `self.PlayerSpotted` (`|CreateDelegate` :!event `PlayerSpotted_Event`))
  (add `self.PlayerLost` (`|CreateDelegate` :!event `PlayerLost_Event`))
  (for _array_element (`PrimitiveComponent.GetOverlappingActors` (`self.CommunicationSphere`) null)
    (bind _aspatrol_guard (cast `/Game/Blueprints/NPC_Blueprints/PatrolGuard` _array_element))
    (`KismetArrayLibrary.Array_AddUnique` (`self.PatrolGuardsInRange`) _aspatrol_guard))
  (`FMODAudioComponent.Stop` (`self.CameraBeep`))
  (bind (_direction _rotationtrack) (`Timeline|RotationTImeline` :!label _label)
    (:`Update`
      (`SceneComponent.K2_SetRelativeRotation` (`self.Head`) (`KismetMathLibrary.MakeRotator` 0.0 0.0 (`KismetMathLibrary.MapRangeClamped` _rotationtrack 0.0 1.0 (`self.RotationStart`) (`self.RotationEnd`))) false false))
    (:`Finished`
      (`/Engine/EditorBlueprintResources/StandardMacros.FlipFlop`
        (:`A`
          (goto _label :!via `ReverseFromEnd`))
        (:`B`
          (goto _label :!via `PlayFromStart`))))))

(event `PlayerSpotted_Event`
  (for _array_element (`self.PatrolGuardsInRange`)
    (`self.AddSightSource` _array_element self))
  (`FMODAudioComponent.Play` (`self.CameraBeep`)))

(event `PlayerLost_Event`
  (for _array_element (`self.PatrolGuardsInRange`)
    (`self.RemoveSightSource` _array_element self))
  (`FMODAudioComponent.Stop` (`self.CameraBeep`)))

(event `self.CommunicationSphere.OnComponentBeginOverlap`
  (params (OverlappedComponent :type "PrimitiveComponent Object Reference") (OtherActor :type "Actor Object Reference") (OtherComp :type "PrimitiveComponent Object Reference") (OtherBodyIndex :type Integer) (bFromSweep :type Boolean) (SweepResult :type "HitResult Structure (by ref)"))
  (bind _aspatrol_guard (cast `/Game/Blueprints/NPC_Blueprints/PatrolGuard` OtherActor))
  (`KismetArrayLibrary.Array_AddUnique` (`self.PatrolGuardsInRange`) _aspatrol_guard)
  (if (`self.HasSeenPlayer`)
    (`self.AddSightSource` _aspatrol_guard self)))

(event `self.CommunicationSphere.OnComponentEndOverlap`
  (params (OverlappedComponent :type "PrimitiveComponent Object Reference") (OtherActor :type "Actor Object Reference") (OtherComp :type "PrimitiveComponent Object Reference") (OtherBodyIndex :type Integer))
  (bind _patrolguardsinrange (`self.PatrolGuardsInRange`))
  (bind _aspatrol_guard (cast `/Game/Blueprints/NPC_Blueprints/PatrolGuard` OtherActor))
  (if (`KismetArrayLibrary.Array_Contains` _patrolguardsinrange _aspatrol_guard)
    (`KismetArrayLibrary.Array_RemoveItem` _patrolguardsinrange _aspatrol_guard)
    (if (`self.HasSeenPlayer`)
      (`self.RemoveSightSource` _aspatrol_guard self))))

(fn `GetEyeTransform`
  (returns (EyeTransform :type "Transform Structure"))
  (return (`SceneComponent.GetSocketTransform` (`self.Head`) "lens" "RTS_World")))

(fn `UserConstructionScript`
  (`SphereComponent.SetSphereRadius` (`self.CommunicationSphere`) (`self.CommunicationRange`) true)
  (set `self.CustomTimeDilation` (`self.RotationSpeedMultiplier`)))