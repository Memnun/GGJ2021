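; Prototype guard base actor that tracks whether the player is seen and visualizes the guard's field of view.
; It keeps a unique list of sight sources, calling PlayerSpotted when the first is added and PlayerLost when the last is removed.
; Every tick it draws a short-lived debug cone from GetEyeTransform, which returns the actor transform, sized by vision distance and angle.
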(event `self.ReceiveTick`
  (params (DeltaSeconds :type "Float (single-precision)"))
  (`KismetSystemLibrary.DrawDebugConeInDegrees` (.location (`self.GetEyeTransform`)) (`KismetMathLibrary.GetForwardVector` (.rotation (`self.GetEyeTransform`))) (`self.VisionDistance`) (* (`self.VisionAngle`) 0.5) 10.0 12 (struct :`R` 1.0 :`G` 0.319207 :`A` 0.5) 0.034 5.0))

(fn `AddSightSource`
  (params (Source :type "Actor Object Reference"))
  (`KismetArrayLibrary.Array_AddUnique` (`self.SightSources`) Source)
  (if (== (`KismetArrayLibrary.Array_Length` (`self.SightSources`)) 1)
    (`self.PlayerSpotted`)))

(fn `GetEyeTransform`
  (returns (EyeTransform :type "Transform Structure"))
  (return (`self.GetTransform`)))

(fn `HasSeenPlayer`
  (returns (Seen :type Boolean))
  (return (> (`KismetArrayLibrary.Array_Length` (`self.SightSources`)) 0)))

(fn `RemoveSightSource`
  (params (Source :type "Actor Object Reference"))
  (bind _sightsources (`self.SightSources`))
  (if (`KismetArrayLibrary.Array_Contains` _sightsources Source)
    (`KismetArrayLibrary.Array_RemoveItem` _sightsources Source)
    (if (== (`KismetArrayLibrary.Array_Length` _sightsources) 0)
      (`self.PlayerLost`))))

(fn `UserConstructionScript`)